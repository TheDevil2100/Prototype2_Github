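; BP_BulletCase is a bullet casing actor that plays an impact sound when its mesh hits something.
; The construction script applies the spawn-provided mesh, which needs simple collision for physics, and picks the bullet or shell impact sound by comparing that mesh.
; On each component hit, it passes that sound to HitImpactSound with close-by attenuation and a pitch range for variation.
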(event OnComponentHit(StaticMesh)
  (params (HitComponent :type Primitive%20Component%20Object%20Reference) (OtherActor :type Actor%20Object%20Reference) (OtherComp :type Primitive%20Component%20Object%20Reference) (NormalImpulse :type Vector :default "0, 0, 0") (Hit :type Hit%20Result%20Structure%20%28by%20ref%29))
  ;[0 0 0] Hit impact sounds
  (Utilities|HitImpactSound (Variables|Default|GetStaticMesh) (Variables|Default|GetImpactSound) "/Game/BossBattles/Blueprint/FPSK/Sounds/Audio/Attenuation_CloseBy.Attenuation_CloseBy" 1.0 1.2))

(fn ConstructionScript
  ;[0 0 0] Set mesh of bullet case from spawn
  (Components|StaticMesh|SetStaticMesh (Variables|Default|GetStaticMesh) (Variables|Default|GetBulletCaseMesh)) ; Make sure mesh is using simple collision for physics
  ;[0 0 0] Set impact sound based on bullet casing mesh
  (Utilities|FlowControl|Sequence
    (:then_0
      (if (== (Variables|Default|GetBulletCaseMesh) "/Game/BossBattles/Blueprint/FPSK/Meshes/SM_BulletCase.SM_BulletCase")
        (Variables|Default|SetImpactSound "/Game/BossBattles/Blueprint/FPSK/Sounds/WAV_BulletCaseImpact.WAV_BulletCaseImpact")))
    (:then_1
      (if (== (Variables|Default|GetBulletCaseMesh) "/Game/BossBattles/Blueprint/FPSK/Meshes/SM_ShellCase.SM_ShellCase")
        (Variables|Default|SetImpactSound "/Game/BossBattles/Blueprint/FPSK/Sounds/WAV_ShellImpact.WAV_ShellImpact")))))