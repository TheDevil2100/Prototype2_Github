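; A destructible TV prop with a flickering screen light and a power cable built at construction.
; The first point damage on a glass surface plays a crackle, stops the flash, destroys the light and swaps in a broken screen material.
; The ScreenFlash timeline lerps light intensity between its default and half.
; The construction script snaps the spline's end to an optional wire socket actor and sweeps spline meshes along it.
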(event Custom|Stop%20animation
  (bind _defaultlightintensity (Variables|Default|GetDefaultLightIntensity))
  ;[0 0 0] Light Animation
  ;;[1 1 1] Light flash animation
  (bind _flashvalue (Timeline|ScreenFlash Stop)
    (:Update
      ;;[1 1 1] Only continue if TV is not destroyed
      (Utilities|IsValid (Variables|Default|GetPointLight)
        (:Is%20Valid
          ;;[1 1 1] Flash between light intensity and half value
          (Rendering|Components|Light|SetIntensity (Variables|Default|GetPointLight) (Math|Float|Lerp _defaultlightintensity (/ _defaultlightintensity 2.0) _flashvalue)))))))

(event Game|Damage|EventPointDamage
  (params (Damage :type Float%20%28single-precision%29) (DamageType :type Damage%20Type%20Object%20Reference) (HitLocation :type Vector :default "0, 0, 0") (HitNormal :type Vector :default "0, 0, 0") (HitComponent :type Primitive%20Component%20Object%20Reference) (BoneName :type Name :default "None") (ShotFromDirection :type Vector :default "0, 0, 0") (InstigatedBy :type Controller%20Object%20Reference) (DamageCauser :type Actor%20Object%20Reference) (HitInfo :type Hit%20Result%20Structure%20%28by%20ref%29))
  ;[0 0 0] TV Destruction logic
  ;;[1 1 1] If shot anywhere on screen
  (if (Utilities|Select :Index (Variables|/Script/Engine.PhysicalMaterial|GetSurfaceType (.PhysMat (Collision|BreakHitResult HitInfo))) :SurfaceType_Default false :SurfaceType1 false :SurfaceType2 false :SurfaceType3 false :SurfaceType4 true :SurfaceType5 false :SurfaceType6 false :SurfaceType7 false :SurfaceType8 false :SurfaceType9 false :SurfaceType10 true :SurfaceType11 false :SurfaceType12 false :SurfaceType13 false :SurfaceType14 false :SurfaceType15 false)
    ;;[1 1 1] Smash TV by playing sound, destroying light and setting broken screen material
    (Utilities|FlowControl|DoOnce false
      (:Completed
        (Audio|PlaySoundatLocation "/Game/BossBattles/Blueprint/FPSK/Sounds/WAV_Electric_Crackle.WAV_Electric_Crackle" (Transformation|GetActorLocation) "0, 0, 0" 1.0 1.0 0.0 "/Game/BossBattles/Blueprint/FPSK/Sounds/Audio/Attenuation_MediumRange.Attenuation_MediumRange" 0 0)
        (CallFunction|StopAnimation)
        (Components|DestroyComponent (Variables|Default|GetPointLight))
        (Rendering|Material|SetMaterial (Variables|Default|GetStaticMesh) 0 "/Game/BossBattles/Blueprint/FPSK/Materials/TV/M_BrokenScreen.M_BrokenScreen")))))

(fn ConstructionScript
  ;[0 0 0] TV Construction
  (Utilities|FlowControl|Sequence
    (:then_0
      ;;[1 1 1] Set default light intensity for flash animation
      (Variables|Default|SetDefaultLightIntensity (Variables|/Script/Engine.LightComponentBase|GetIntensity (Variables|Default|GetPointLight))))
    (:then_1
      ;;[1 1 1] If there is a wire socket refence
      (Utilities|IsValid (Variables|Default|GetWireSocketReference)
        (:Is%20Valid
          ;;[1 1 1] Set final spline point to socket reference if valid
          (Spline|SetLocationatSplinePoint (Variables|Default|GetSpline) (- (Spline|GetNumberOfSplinePoints (Variables|Default|GetSpline)) 1) (Transformation|GetActorLocation (Variables|Default|GetWireSocketReference)) "World" true))))
    (:then_2
      ;;[1 1 1] For each spline point
      (for _index (range 0 (- (Spline|GetNumberOfSplinePoints (Variables|Default|GetSpline)) 2))
        (Variables|Default|SetSpline%20Index _index)
        ;;[1 1 1] Add spline mesh component
        (bind _returnvalue (AddComponent|AddSplineMeshComponent false (Transformation|GetRelativeTransform (Variables|Default|GetSpline))))
        ;;[1 1 1] Sweep wire mesh along the spline
        (SplineMesh|SetStartandEnd _returnvalue (.Location (Spline|GetLocationandTangentatSplinePoint (Variables|Default|GetSpline) (Variables|Default|GetSpline%20Index) "Local")) (.Tangent (Spline|GetLocationandTangentatSplinePoint (Variables|Default|GetSpline) (Variables|Default|GetSpline%20Index) "Local")) (.Location (Spline|GetLocationandTangentatSplinePoint (Variables|Default|GetSpline) (+ (Variables|Default|GetSpline%20Index) 1) "Local")) (.Tangent (Spline|GetLocationandTangentatSplinePoint (Variables|Default|GetSpline) (+ (Variables|Default|GetSpline%20Index) 1) "Local")) true :!class /Script/Engine.SplineMeshComponent)))))