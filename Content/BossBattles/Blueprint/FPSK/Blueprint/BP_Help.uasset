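; Help marker actor that types its help text into the player's HUD subtitle while a FirstPersonCharacter overlaps its box.
; BuildNextLetter re-calls itself after a tiny delay to append one character at a time, treating any "{" as a whole "{br}" line-break token.
; Leaving the box stops the build and clears the subtitle.
; The construction script colours both text renders; the marker's float-and-spin timeline logic is never run.
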(event OnComponentBeginOverlap(Box)
  (params (OverlappedComponent :type Primitive%20Component%20Object%20Reference) (OtherActor :type Actor%20Object%20Reference) (OtherComp :type Primitive%20Component%20Object%20Reference) (OtherBodyIndex :type Integer) (bFromSweep :type Boolean) (SweepResult :type Hit%20Result%20Structure%20%28by%20ref%29))
  (bind _helptext (Variables|Default|GetHelpText))
  (bind _returnvalue (Utilities|String|ToString(Text) _helptext))
  (bind _returnvalue_2 (Utilities|String|GetCharacterArrayfromString _returnvalue))
  ;[0 0 0] Overlap events
  (bind _asfirst_person_character (Utilities|Casting|CastToFirstPersonCharacter OtherActor))
  ;;[1 1 1] Set character reference and show subtitle in player HUD
  (bind _output_get (Variables|Default|SetCharacterReference_Overlap _asfirst_person_character))
  (Utilities|IsValid (Variables|/Game/BossBattles/Blueprint/FPSK/FirstPersonAssets/FirstPersonBP/Blueprints/FirstPersonCharacter.FirstPersonCharacter_C|GetMainHUD _output_get)
    (:Is%20Valid
      (Variables|/Game/BossBattles/Blueprint/FPSK/Blueprint/Widget/BP_MainHUD.BP_MainHUD_C|SetShowSubtitle (Variables|/Game/BossBattles/Blueprint/FPSK/FirstPersonAssets/FirstPersonBP/Blueprints/FirstPersonCharacter.FirstPersonCharacter_C|GetMainHUD _output_get) true)
      ;;[1 1 1] Allow text building
      (Variables|Default|SetContinueBuild true)
      ;;[1 1 1] Reset built text and current letter index
      (Variables|Default|SetBuiltText "")
      (Variables|Default|SetLetterIndex 0)
      ;[0 0 0] Build text
      ;;[1 1 1] Only if continue build is true(So text stops building on end overlap)
      (if (Variables|Default|GetContinueBuild)
        ;;[1 1 1] Only continue if built text is not complete
        (if (< (Utilities|Array|Length (Utilities|String|GetCharacterArrayfromString (Variables|Default|GetBuiltText))) (Utilities|Array|Length _returnvalue_2))
          ;;[1 1 1] Build text with new letter/s
          (Variables|Default|SetBuiltText (Utilities|String|Append (Variables|Default|GetBuiltText) (Utilities|String|SelectString "{br}" (Utilities|Array|Get(acopy) _returnvalue_2 (Variables|Default|GetLetterIndex)) (Utilities|Enum|Equal(Enum) (Utilities|Array|Get(acopy) _returnvalue_2 (Variables|Default|GetLetterIndex)) "{"))))
          ;;[1 1 1] Increase letter index
          (Variables|Default|SetLetterIndex (+ (Variables|Default|GetLetterIndex) (Math|Integer|SelectInt 4 1 (Utilities|Enum|Equal(Enum) (Utilities|Array|Get(acopy) _returnvalue_2 (Variables|Default|GetLetterIndex)) "{"))))
          ;;[1 1 1] Set text built text in HUD
          (Default|PlaySubtitle (Variables|/Game/BossBattles/Blueprint/FPSK/FirstPersonAssets/FirstPersonBP/Blueprints/FirstPersonCharacter.FirstPersonCharacter_C|GetMainHUD (Variables|Default|GetCharacterReference_Overlap)) (Utilities|Text|ToText(String) (Variables|Default|GetBuiltText)) 0.0)
          ;;[1 1 1] Delay and build next letter
          (Utilities|FlowControl|Delay 0.001) ; Text Speed
          (CallFunction|BuildNextLetter))))))

(event OnComponentEndOverlap(Box)
  (params (OverlappedComponent :type Primitive%20Component%20Object%20Reference) (OtherActor :type Actor%20Object%20Reference) (OtherComp :type Primitive%20Component%20Object%20Reference) (OtherBodyIndex :type Integer))
  ;[0 0 0] End Overlap Events
  (bind _asfirst_person_character (Utilities|Casting|CastToFirstPersonCharacter OtherActor))
  ;;[1 1 1] Set character reference and hide subtitle
  (bind _output_get (Variables|Default|SetCharacterReference_EndOverlap _asfirst_person_character))
  (Utilities|IsValid (Variables|/Game/BossBattles/Blueprint/FPSK/FirstPersonAssets/FirstPersonBP/Blueprints/FirstPersonCharacter.FirstPersonCharacter_C|GetMainHUD _output_get)
    (:Is%20Valid
      (Variables|/Game/BossBattles/Blueprint/FPSK/Blueprint/Widget/BP_MainHUD.BP_MainHUD_C|SetShowSubtitle (Variables|/Game/BossBattles/Blueprint/FPSK/FirstPersonAssets/FirstPersonBP/Blueprints/FirstPersonCharacter.FirstPersonCharacter_C|GetMainHUD _output_get) false)
      (Variables|/Game/BossBattles/Blueprint/FPSK/Blueprint/Widget/BP_MainHUD.BP_MainHUD_C|SetSubtitleTextContent (Variables|/Game/BossBattles/Blueprint/FPSK/FirstPersonAssets/FirstPersonBP/Blueprints/FirstPersonCharacter.FirstPersonCharacter_C|GetMainHUD _output_get) "")
      ;;[1 1 1] Disable Text building
      (Variables|Default|SetContinueBuild false)
      ;;[1 1 1] Reset text build variables
      (Variables|Default|SetBuiltText "")
      (Variables|Default|SetLetterIndex 0))))

(event Custom|BuildNextLetter
  (bind _helptext (Variables|Default|GetHelpText))
  (bind _returnvalue (Utilities|String|ToString(Text) _helptext))
  (bind _returnvalue_2 (Utilities|String|GetCharacterArrayfromString _returnvalue))
  ;[0 0 0] Build text
  ;;[1 1 1] Only if continue build is true(So text stops building on end overlap)
  (if (Variables|Default|GetContinueBuild)
    ;;[1 1 1] Only continue if built text is not complete
    (if (< (Utilities|Array|Length (Utilities|String|GetCharacterArrayfromString (Variables|Default|GetBuiltText))) (Utilities|Array|Length _returnvalue_2))
      ;;[1 1 1] Build text with new letter/s
      (Variables|Default|SetBuiltText (Utilities|String|Append (Variables|Default|GetBuiltText) (Utilities|String|SelectString "{br}" (Utilities|Array|Get(acopy) _returnvalue_2 (Variables|Default|GetLetterIndex)) (Utilities|Enum|Equal(Enum) (Utilities|Array|Get(acopy) _returnvalue_2 (Variables|Default|GetLetterIndex)) "{"))))
      ;;[1 1 1] Increase letter index
      (Variables|Default|SetLetterIndex (+ (Variables|Default|GetLetterIndex) (Math|Integer|SelectInt 4 1 (Utilities|Enum|Equal(Enum) (Utilities|Array|Get(acopy) _returnvalue_2 (Variables|Default|GetLetterIndex)) "{"))))
      ;;[1 1 1] Set text built text in HUD
      (Default|PlaySubtitle (Variables|/Game/BossBattles/Blueprint/FPSK/FirstPersonAssets/FirstPersonBP/Blueprints/FirstPersonCharacter.FirstPersonCharacter_C|GetMainHUD (Variables|Default|GetCharacterReference_Overlap)) (Utilities|Text|ToText(String) (Variables|Default|GetBuiltText)) 0.0)
      ;;[1 1 1] Delay and build next letter
      (Utilities|FlowControl|Delay 0.001) ; Text Speed
      (CallFunction|BuildNextLetter))))

(fn ConstructionScript
  ;[0 0 0] Set text render color
  (Rendering|Components|TextRender|SetTextRenderColor (Variables|Default|GetTextRender_Mirror) (Variables|Default|GetIconColor)))