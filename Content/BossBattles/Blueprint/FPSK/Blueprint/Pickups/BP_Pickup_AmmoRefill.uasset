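; Ammo refill pickup that restores clip and reserve ammo to maximum for every weapon in the player's inventory.
; On PickupEffect it first checks whether any weapon is below full clip or reserve ammo.
; If so, it rebuilds each inventory weapon struct with both counts maxed and calls PickupEvent.
; Otherwise, it shows an "Ammo is already full" HUD subtitle and skips the pickup event.
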(event Custom|BreakAmmoCheck
  ;[0 0 0] Check if ammo isn't already full
  (Utilities|Array|ForEachLoopwithBreak (Variables|/Game/BossBattles/Blueprint/FPSK/FirstPersonAssets/FirstPersonBP/Blueprints/FirstPersonCharacter.FirstPersonCharacter_C|Get[Inventory]WeaponInventory (Variables|Default|GetCharacterReference))) ; enters at Break
)

(event EventPickupEffect
  ;[0 0 0] Check if ammo isn't already full
  (bind _array_element (Utilities|Array|ForEachLoopwithBreak (Variables|/Game/BossBattles/Blueprint/FPSK/FirstPersonAssets/FirstPersonBP/Blueprints/FirstPersonCharacter.FirstPersonCharacter_C|Get[Inventory]WeaponInventory (Variables|Default|GetCharacterReference)))
    (:LoopBody
      (if (or (!= (.ClipSize (Utilities|Struct|BreakStruct_WeaponVariables _array_element)) (.ClipAmmo (Utilities|Struct|BreakStruct_WeaponVariables _array_element))) (!= (.MaxAmmo (Utilities|Struct|BreakStruct_WeaponVariables _array_element)) (.Ammo (Utilities|Struct|BreakStruct_WeaponVariables _array_element))))
        (Variables|Default|SetAmmoIsNotFull true)))
    (:Completed
      ;[0 0 0] Continue only if character needs ammo
      (if (Variables|Default|GetAmmoIsNotFull)
        ;[0 0 0] Refill all ammo in current inventory
        (for (_array_element_2 _array_index) (Variables|/Game/BossBattles/Blueprint/FPSK/FirstPersonAssets/FirstPersonBP/Blueprints/FirstPersonCharacter.FirstPersonCharacter_C|Get[Inventory]WeaponInventory (Variables|Default|GetCharacterReference))
          (Utilities|Array|SetArrayElem (Variables|/Game/BossBattles/Blueprint/FPSK/FirstPersonAssets/FirstPersonBP/Blueprints/FirstPersonCharacter.FirstPersonCharacter_C|Get[Inventory]WeaponInventory (Variables|Default|GetCharacterReference)) _array_index (Utilities|Struct|MakeStruct_WeaponVariables (.WeaponMesh (Utilities|Struct|BreakStruct_WeaponVariables _array_element_2)) (.Material (Utilities|Struct|BreakStruct_WeaponVariables _array_element_2)) (.BulletCasingMesh (Utilities|Struct|BreakStruct_WeaponVariables _array_element_2)) (.WeaponAnimationBP (Utilities|Struct|BreakStruct_WeaponVariables _array_element_2)) (.ArmAnimationBP (Utilities|Struct|BreakStruct_WeaponVariables _array_element_2)) (.AnimationSet (Utilities|Struct|BreakStruct_WeaponVariables _array_element_2)) (.WeaponName (Utilities|Struct|BreakStruct_WeaponVariables _array_element_2)) (.WeaponType (Utilities|Struct|BreakStruct_WeaponVariables _array_element_2)) (.Sights (Utilities|Struct|BreakStruct_WeaponVariables _array_element_2)) (.SightSettings (Utilities|Struct|BreakStruct_WeaponVariables _array_element_2)) (.MuzzleAttachment (Utilities|Struct|BreakStruct_WeaponVariables _array_element_2)) (.Foregrip (Utilities|Struct|BreakStruct_WeaponVariables _array_element_2)) (.ShootSound (Utilities|Struct|BreakStruct_WeaponVariables _array_element_2)) (.MinSoundPitch (Utilities|Struct|BreakStruct_WeaponVariables _array_element_2)) (.MaxSoundPitch (Utilities|Struct|BreakStruct_WeaponVariables _array_element_2)) (.Damage (Utilities|Struct|BreakStruct_WeaponVariables _array_element_2)) (.PenetrationPower (Utilities|Struct|BreakStruct_WeaponVariables _array_element_2)) (.Firerate (Utilities|Struct|BreakStruct_WeaponVariables _array_element_2)) (.ReloadSpeed (Utilities|Struct|BreakStruct_WeaponVariables _array_element_2)) (.ADSSpeed (Utilities|Struct|BreakStruct_WeaponVariables _array_element_2)) (.Mobility (Utilities|Struct|BreakStruct_WeaponVariables _array_element_2)) (.AimMobilityMultiplier (Utilities|Struct|BreakStruct_WeaponVariables _array_element_2)) (.SprintMobilityMultiplier (Utilities|Struct|BreakStruct_WeaponVariables _array_element_2)) (.CrouchMobilityMultiplier (Utilities|Struct|BreakStruct_WeaponVariables _array_element_2)) (.ProneMobilityMultiplier (Utilities|Struct|BreakStruct_WeaponVariables _array_element_2)) (.Range (Utilities|Struct|BreakStruct_WeaponVariables _array_element_2)) (.Recoil (Utilities|Struct|BreakStruct_WeaponVariables _array_element_2)) (.RecoilCooldownRate (Utilities|Struct|BreakStruct_WeaponVariables _array_element_2)) (.Spread (Utilities|Struct|BreakStruct_WeaponVariables _array_element_2)) (.HipfireRecoilMultiplier (Utilities|Struct|BreakStruct_WeaponVariables _array_element_2)) (.InitialHipfireSpread (Utilities|Struct|BreakStruct_WeaponVariables _array_element_2)) (.InitialADSSpread (Utilities|Struct|BreakStruct_WeaponVariables _array_element_2)) (.ShotgunPellets (Utilities|Struct|BreakStruct_WeaponVariables _array_element_2)) (.BurstAmount (Utilities|Struct|BreakStruct_WeaponVariables _array_element_2)) (.BurstCooldown (Utilities|Struct|BreakStruct_WeaponVariables _array_element_2)) (.ClipSize (Utilities|Struct|BreakStruct_WeaponVariables _array_element_2)) (.MaxAmmo (Utilities|Struct|BreakStruct_WeaponVariables _array_element_2)) (.ClipSize (Utilities|Struct|BreakStruct_WeaponVariables _array_element_2)) (.MaxAmmo (Utilities|Struct|BreakStruct_WeaponVariables _array_element_2)))))
        ;;[1 1 1] Play pickup event
        (CallFunction|PickupEvent)
        (else
          ;;[1 1 1] Notifiy player ammo is already full
          (Default|PlaySubtitle (Variables|/Game/BossBattles/Blueprint/FPSK/FirstPersonAssets/FirstPersonBP/Blueprints/FirstPersonCharacter.FirstPersonCharacter_C|GetMainHUD (Variables|Default|GetCharacterReference)) "Ammo is already full." 2.0))))))

(fn ConstructionScript
  (|CallParentFunction))