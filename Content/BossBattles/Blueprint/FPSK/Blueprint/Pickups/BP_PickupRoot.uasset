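; Base pickup actor that detects an overlapping FirstPersonCharacter and hands off to PickupEffect, an empty event for child classes to implement.
; Construction applies mesh, light and particle settings; optional timeline-driven hover and spin also enables an obstruction check before pickup.
; PickupEvent, not called here, hides the mesh and light with a sound, then destroys the actor or restores it after a respawn delay.
; An optional lifetime destroys the pickup automatically.
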(event OnComponentBeginOverlap(Sphere)
  (params (OverlappedComponent :type Primitive%20Component%20Object%20Reference) (OtherActor :type Actor%20Object%20Reference) (OtherComp :type Primitive%20Component%20Object%20Reference) (OtherBodyIndex :type Integer) (bFromSweep :type Boolean) (SweepResult :type Hit%20Result%20Structure%20%28by%20ref%29))
  ;[0 0 0] Pickup event
  ;;[1 1 1] Initial overlap and character set
  (bind _asfirst_person_character (Utilities|Casting|CastToFirstPersonCharacter OtherActor))
  (if (Rendering|IsVisible (Variables|Default|GetStaticMesh))
    (bind _output_get (Variables|Default|SetCharacterReference _asfirst_person_character))
    (if (Variables|PickupSettings|GetFloatAnimation)
      ;;[1 1 1] Check if anything is between you and pickup eg: a wall
      (Utilities|ObstructionCheck self _output_get
        (:No%20Obstruction
          ;;[1 1 1] Set events that pickup performs
          (CallFunction|PickupEffect :!label _label))
        (:Blocked
          (Variables|Default|SetCharacterReference 0)))
      (else
        (goto _label)))))

(event Custom|PickupEffect
  ;[0 0 0] Pickup Effect (Continues to child classes)
)

(event Custom|PlayFloatAnimation
  (bind _returnvalue (Transformation|GetActorLocation))
  (bind (_x _y) (Math|Vector|BreakVector _returnvalue))
  ;[0 0 0] Float Animation
  (bind _zfloat (Timeline|PickupFloatAnimation PlayFromStart)
    (:Update
      ;;[1 1 1] Set pickup location and rotation
      (Transformation|SetActorLocation (Math|Vector|MakeVector _x _y (+ (* _zfloat 1e+01) (Variables|Default|GetInitialZLocation))) false false)
      (Class|Actor|AddActorWorldRotation (Math|Rotator|MakeRotator 0.0 0.0 (Variables|PickupSettings|GetRotationSpeed))))))

(event Custom|DestroyCountdown
  ;[0 0 0] Destroy pickup
  (Utilities|FlowControl|Delay (Variables|PickupSettings|GetPickupLifetime))
  (Actor|DestroyActor))

(event Custom|PickupEvent
  ;[0 0 0] When picked up, activate respawn timer or destroy pickup
  ;;[1 1 1] Hide pickup
  (CallFunction|Hide/ShowPickup true)
  (if (Variables|PickupSettings|GetDestroyOnPickup)
    ;;[1 1 1] Destroy pickup
    (Actor|DestroyActor)
    (else
      ;;[1 1 1] Wait respawn duration
      (Utilities|FlowControl|Delay (Variables|PickupSettings|GetPickupRespawnTime))
      ;;[1 1 1] Show pickup
      (CallFunction|Hide/ShowPickup false))))

(event EventBeginPlay
  ;[0 0 0] Begin play
  (Utilities|FlowControl|Sequence
    (:then_0
      (if (Variables|PickupSettings|GetFloatAnimation) ; Play float animation if true
        (CallFunction|PlayFloatAnimation)))
    (:then_1
      (if (> (Variables|PickupSettings|GetPickupLifetime) 0.0) ; Destroy pickup  if duration more than 0
        (CallFunction|DestroyCountdown)))))

(fn ConstructionScript
  ;[0 0 0] Set mesh, light color and light intensity on construction
  (Components|StaticMesh|SetStaticMesh (Variables|Default|GetStaticMesh) (Variables|PickupSettings|GetPickupMesh))
  (Rendering|Components|Light|SetLightColor (Variables|Default|GetPointLight) (Variables|PickupSettings|GetLightColor) true)
  (Effects|Components|ParticleSystem|SetTemplate (Variables|Default|GetParticleSystem) (Variables|PickupSettings|GetParticle))
  (Variables|PickupSettings|SetLightIntensity (Variables|/Script/Engine.LightComponentBase|GetIntensity (Variables|Default|GetPointLight)))
  ;[0 0 0] Set Initial Z location
  (Variables|Default|SetInitialZLocation (.Z (Math|Vector|BreakVector (Transformation|GetActorLocation)))))

(fn Hide/ShowPickup
  (params (Hide :type Boolean))
  ;[1 1 1] Show/Hide mesh and light
  (Rendering|SetVisibility (Variables|Default|GetStaticMesh) (select Hide false true) false)
  (Rendering|Components|Light|SetIntensity (Variables|Default|GetPointLight) (select Hide 0.0 (Variables|PickupSettings|GetLightIntensity)))
  ;[1 1 1] If hiding, play sound
  (if Hide
    ;[1 1 1] Play sound
    (Audio|PlaySound2D (Variables|PickupSettings|GetPickupSound) 1.0 1.0 0.0 0 0)))