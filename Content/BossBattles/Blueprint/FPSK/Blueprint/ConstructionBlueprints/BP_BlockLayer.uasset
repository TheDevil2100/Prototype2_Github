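; BP_BlockLayer is a construction-time tool that lays a row of framed blocks along the actor's forward vector.
; The horizontal length of LayeringEndPoint divided by Spacing sets the block count and stretches a structure mesh, whose TilingV material parameter follows that length.
; Each step adds a static or destructible block, chosen by UseDestructibleMesh and given the selected Material, plus an instanced frame mesh.
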(fn ConstructionScript
  (bind _layeringendpoint (Variables|Default|GetLayeringEndPoint))
  (bind (_x _y) (Math|Vector|BreakVector _layeringendpoint))
  ;[0 0 0] Construct block layers
  ;;[1 1 1] Set number of blocks based on end point and spacing
  (Variables|Default|SetNumberOfBlocks (Math|Float|Truncate (/ (Math|Vector|VectorLength (Math|Vector|MakeVector _x _y 0.0)) (Variables|Default|GetSpacing))))
  ;;[1 1 1] Create instances of block frames
  (bind _returnvalue (AddComponent|AddInstancedStaticMeshComponent true (Math|Transform|MakeTransform (Transformation|GetActorLocation) (Transformation|GetActorRotation))))
  (bind _output_get (Variables|Default|SetBlockFrames _returnvalue))
  (Components|StaticMesh|SetStaticMesh _output_get (Variables|Default|GetFrameMesh))
  ;;[1 1 1] Create structure, scaled based on number of blocks and spacing
  (bind _returnvalue_2 (AddComponent|AddStaticMeshComponent false (Math|Transform|MakeTransform "0, 0, 0" (Transformation|GetActorRotation) (Math|Vector|MakeVector (* (Variables|Default|GetNumberOfBlocks) (Variables|Default|GetSpacing)) 1.0 1.0))))
  ;;[1 1 1] Fix UV of frame structure
  (Rendering|Material|SetScalarParameterValueonMaterials _returnvalue_2 "TilingV" (* (Variables|Default|GetNumberOfBlocks) (Variables|Default|GetSpacing)))
  ;;[1 1 1] Loop block construction
  (for _index (range 0 (Variables|Default|GetNumberOfBlocks))
    (Variables|Default|SetLoopIndex _index)
    ;;[1 1 1] Whether to use standard or destructible mesh block
    (if (Variables|Default|GetUseDestructibleMesh)
      ;;[1 1 1] Add destructible mesh
      (bind _returnvalue_3 (AddComponent|AddActorComponent false (Math|Transform|MakeTransform (* (* (Math|Vector|GetForwardVector (Transformation|GetActorRotation)) (Variables|Default|GetSpacing)) (Variables|Default|GetLoopIndex)) (Transformation|GetActorRotation))))
      (bind _output_get_2 (Variables|Default|SetDestructibleMesh 0 _returnvalue_3))
      ;;[1 1 1] Set selected material for all elements
      (for _index_2 (range 0 (- (Rendering|Material|GetNumMaterials _output_get_2) 1))
        (Rendering|Material|SetMaterial (.DestructibleMesh (Variables|Default|GetDestructibleMesh)) _index_2 (Variables|Default|GetMaterial)))
      (else
        ;;[1 1 1] Add static mesh
        (bind _returnvalue_4 (AddComponent|AddStaticMeshComponent false (Math|Transform|MakeTransform (* (* (Math|Vector|GetForwardVector (Transformation|GetActorRotation)) (Variables|Default|GetSpacing)) (Variables|Default|GetLoopIndex)) (Transformation|GetActorRotation))))
        ;;[1 1 1] Set selected material
        (Rendering|Material|SetMaterial _returnvalue_4 0 (Variables|Default|GetMaterial))))
    ;;[1 1 1] Add frame to each block
    (Components|InstancedStaticMesh|AddInstance (Variables|Default|GetBlockFrames) (Math|Transform|MakeTransform (* (* (Math|Vector|GetForwardVector (Transformation|GetActorRotation)) (Variables|Default|GetSpacing)) (Variables|Default|GetLoopIndex)) (Transformation|GetActorRotation)))))