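; BP_Target_2 is an FPS target actor that handles scoring, player targeting and pickup drops.
; AddScore and DeductScore update the character's HUD score and multiplier, gated so that during a course only its initiator scores on course targets.
; GetClosestCharacter scans living FirstPersonCharacters by distance to set FollowTarget.
; DropMacro rolls a percentage chance to spawn a timed pickup randomly around the target, optionally allowing multiple drops.
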(fn ConstructionScript)

(fn DeductScore
  (params (Deducted%20Score :type Integer))
  (bind _characterreference (Variables|Default|GetCharacterReference))
  (bind _mainhud (Variables|/Game/BossBattles/Blueprint/FPSK/FirstPersonAssets/FirstPersonBP/Blueprints/FirstPersonCharacter.FirstPersonCharacter_C|GetMainHUD _characterreference))
  (Utilities|CourseTargetCheck
    (:Output
      (Variables|/Game/BossBattles/Blueprint/FPSK/Blueprint/Widget/BP_MainHUD.BP_MainHUD_C|SetMultiplier _mainhud 0)
      (Variables|/Game/BossBattles/Blueprint/FPSK/Blueprint/Widget/BP_MainHUD.BP_MainHUD_C|SetScore _mainhud (- (Variables|/Game/BossBattles/Blueprint/FPSK/Blueprint/Widget/BP_MainHUD.BP_MainHUD_C|GetScore _mainhud) Deducted%20Score))
      (Default|ScoreDeductEvent _mainhud (Utilities|Text|ToText(String) (Utilities|String|Append "-" (Utilities|String|ToString(Integer) Deducted%20Score)))))))

(fn AddScore
  (params (Added%20Score :type Integer) (Added%20Multiplier :type Integer) (Reset%20Multiplier? :type Boolean))
  (bind _characterreference (Variables|Default|GetCharacterReference))
  (bind _mainhud (Variables|/Game/BossBattles/Blueprint/FPSK/FirstPersonAssets/FirstPersonBP/Blueprints/FirstPersonCharacter.FirstPersonCharacter_C|GetMainHUD _characterreference))
  (Utilities|CourseTargetCheck
    (:Output
      (Variables|/Game/BossBattles/Blueprint/FPSK/Blueprint/Widget/BP_MainHUD.BP_MainHUD_C|SetScoreDisplay _mainhud (+ (Variables|/Game/BossBattles/Blueprint/FPSK/Blueprint/Widget/BP_MainHUD.BP_MainHUD_C|GetScoreDisplay _mainhud) Added%20Score))
      (Variables|/Game/BossBattles/Blueprint/FPSK/Blueprint/Widget/BP_MainHUD.BP_MainHUD_C|SetMultiplier _mainhud (Math|Integer|SelectInt 0 (+ (Variables|/Game/BossBattles/Blueprint/FPSK/Blueprint/Widget/BP_MainHUD.BP_MainHUD_C|GetMultiplier _mainhud) Added%20Multiplier) Reset%20Multiplier?))
      (Default|ScorePopinAnimation _mainhud))))

(fn RefollowCharacter)

(fn GetClosestCharacter
  ;[1 1 1] Clear live players array
  (Utilities|Array|Clear (Variables|Default|GetLivePlayers))
  ;[1 1 1] Add all live players to array
  (bind _outactors (Actor|GetAllActorsOfClass "/Game/BossBattles/Blueprint/FPSK/FirstPersonAssets/FirstPersonBP/Blueprints/FirstPersonCharacter.FirstPersonCharacter_C"))
  (for _array_element _outactors
    (if (not (Variables|/Game/BossBattles/Blueprint/FPSK/FirstPersonAssets/FirstPersonBP/Blueprints/FirstPersonCharacter.FirstPersonCharacter_C|GetDead _array_element))
      (Utilities|Array|Add (Variables|Default|GetLivePlayers) _array_element)))
  ;[1 1 1] If there is any live players found
  (if (> (Utilities|Array|Length (Variables|Default|GetLivePlayers)) 0)
    ;[1 1 1] Set first closest player reference
    (bind _output_get (Variables|Default|SetClosestPlayerReference (Utilities|Array|Get(acopy) (Variables|Default|GetLivePlayers))))
    (Utilities|IsValid _output_get
      (:Is%20Valid
        (Utilities|FlowControl|Sequence
          (:then_0
            ;[1 1 1] Must set first distance check to any player for compare loop
            (Utilities|IsValid (Variables|Default|GetClosestPlayerReference)
              (:Is%20Valid
                (Variables|Default|SetClosestPlayerDistance (Transformation|GetDistanceTo (Variables|Default|GetClosestPlayerReference))))))
          (:then_1
            ;[1 1 1] For all live targets
            (for _array_element_2 (Variables|Default|GetLivePlayers)
              ;[1 1 1] Check if still alive for good measure
              (bind _output_get_2 (Variables|Default|SetClosestPlayerReference _array_element_2))
              (if (not (Variables|/Game/BossBattles/Blueprint/FPSK/FirstPersonAssets/FirstPersonBP/Blueprints/FirstPersonCharacter.FirstPersonCharacter_C|GetDead _output_get_2))
                ;[1 1 1] Check if distance is closer than any previous checks
                (bind _output_get_3 (Variables|Default|SetCurrentPlayerDistance (Transformation|GetDistanceTo (Variables|Default|GetClosestPlayerReference))))
                (Math|Float|CompareFloat _output_get_3 (Variables|Default|GetClosestPlayerDistance)
                  (:==
                    _)
                  (:<
                    _))
                ;[1 1 1] Set Closest player and set Closest Player Distance if closer to target
                (Variables|Default|SetFollowTarget (Variables|Default|GetClosestPlayerReference))
                (Variables|Default|SetClosestPlayerDistance (Variables|Default|GetCurrentPlayerDistance))))))))
    (else
      ;[1 1 1] Set Follow target to none if there are no live targets found
      (Variables|Default|SetFollowTarget 0))))