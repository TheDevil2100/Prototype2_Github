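; Spawn point actor for the zombie game mode that marks where spawning can happen and whether it is currently allowed.
; Each tick it sets CanSpawn to false while a FirstPersonCharacter overlaps its DontSpawnRadius, and true otherwise.
; The construction script stores the actor's location and rotation, with unit scale, as the SpawnLocation transform.
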(event EventTick
  (params (DeltaSeconds :type Float%20%28single-precision%29))
  ;[0 0 0] If there is a player within DontSpawnRadius, not considered for spawning
  (if (> (Utilities|Array|Length (Collision|GetOverlappingActors (Variables|Default|GetDontSpawnRadius) "/Game/BossBattles/Blueprint/FPSK/FirstPersonAssets/FirstPersonBP/Blueprints/FirstPersonCharacter.FirstPersonCharacter_C" :!class /Script/Engine.PrimitiveComponent)) 0)
    (Variables|Default|SetCanSpawn false)
    (else
      (Variables|Default|SetCanSpawn true))))

(fn ConstructionScript
  (bind _returnvalue (Transformation|GetActorTransform))
  (bind (_location _rotation) (Math|Transform|BreakTransform _returnvalue))
  (Variables|Default|SetSpawnLocation (Math|Transform|MakeTransform _location _rotation)))